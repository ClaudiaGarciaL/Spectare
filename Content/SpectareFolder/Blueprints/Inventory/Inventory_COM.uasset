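; Inventory component that holds a fixed number of item slots and toggles an inventory window.
; On BeginPlay it resizes the slot array to its configured space.
; Non-stackable items overwrite the first slot matching an empty zero-quantity struct; stackable items have no handling here.
; OpenClose creates or removes the window widget, placing it center-anchored on the menu player controller's HUD canvas at a stored position.
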(event EventBeginPlay
  (CallFunction|StartInventory))

(fn OpenClose
  (bind _windowinventory (Variables|Default|GetWindowInventory)
    (:then
      (Widget|RemovefromParent _windowinventory)
      (Variables|Default|SetWindowInventory 0))
    (:else
      (bind _returnvalue (UserInterface|CreateWidget "/Game/SpectareFolder/Blueprints/Inventory/WindowInventory.WindowInventory_C" (Game|GetPlayerController 0) self))
      (Variables|Default|SetWindowInventory _returnvalue)
      (bind _asplayer_controller_menu (Utilities|Casting|CastToPlayerController_Menu (Game|GetPlayerController 0)))
      (bind _returnvalue_2 (Class|CanvasPanel|AddChildtoCanvas (Variables|/Game/SpectareFolder/Blueprints/Inventory/HUD.HUD_C|GetHUD (Variables|/Game/SpectareFolder/Blueprints/PlayerController_Menu.PlayerController_Menu_C|GetVariableHUD _asplayer_controller_menu)) (Variables|Default|GetWindowInventory)))
      (Class|CanvasPanelSlot|SetAutoSize _returnvalue_2 true)
      (Class|CanvasPanelSlot|SetAlignment _returnvalue_2 "(X=0.500000,Y=0.500000)")
      (Class|CanvasPanelSlot|SetAnchors _returnvalue_2 (Utilities|Struct|MakeAnchors "(X=0.500000,Y=0.500000)" "(X=0.500000,Y=0.500000)"))
      (Class|CanvasPanelSlot|SetPosition _returnvalue_2 (Variables|Default|GetPosition)))))

(fn AddInventory
  (params (AddContent :type Space%20STR%20Structure))
  (if (not (.esapilable (.objectstructure AddContent)))
    (CallFunction|CreatePlus AddContent)
    (return false)))

(fn StartInventory
  (Utilities|Array|Resize (Variables|Default|GetInventory) (Variables|Default|GetSpace)))

(fn CreatePlus
  (params (AddContent :type Space%20STR%20Structure))
  (bind _inventory (Variables|Default|GetInventory))
  (Utilities|Array|SetArrayElem _inventory (Utilities|Array|FindItem _inventory (Utilities|Struct|MakeSpace_STR "(Name_20_499D8F5C48630822474B15BC6C398083=NSLOCTEXT(\"[4E9E86CB294714001F9C5BBEBDAF31B6]\", \"A7FBD7D8D04EC17B1E7C39BAFEBF9174\", \"Wire\"),EsApilable_5_1AAD764E4156A8142822F1800537C85F=False,Imagen_8_B7649EFF4701A95E5A446CA4B9C9DB3A=None,MaxApilable_16_18CA50E54CDE9AD1D58752AEFC5CAD6A=1,Class_18_015E123D40FA58D16CC27D84F45C9020=None)")) AddContent))