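; Inspectable trophy actor that the player clicks to pull up to the camera, rotate, and read about.
; On click it saves its transform, attaches to the camera manager, tweens into view and enables Turn/LookUp rotation; Cancel detaches and tweens it back.
; While inspecting, it applies depth-of-field through a post-process volume and shows a detail widget with the object's name and description.
; Cursor hover toggles a "Selected" material parameter as a highlight.
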(event OnEndCursorOver(TrophyModel)
  (params (TouchedComponent :type Primitive%20Component%20Object%20Reference))
  ;[1 1 1] Cursor
  (Rendering|Material|SetScalarParameterValueonMaterials (Variables|Default|GetTrophyModel) "Selected" 0.0))

(event OnBeginCursorOver(TrophyModel)
  (params (TouchedComponent :type Primitive%20Component%20Object%20Reference))
  ;[1 1 1] Cursor
  (if (not (Variables|Default|GetInspecting))
    (Rendering|Material|SetScalarParameterValueonMaterials (Variables|Default|GetTrophyModel) "Selected" 1.0)))

(event MouseInput|EventActorOnClicked
  (params (ButtonPressed :type Key%20Structure))
  (bind _returnvalue (Transformation|GetActorTransform))
  (bind _defaultsceneroot (Variables|Default|GetDefaultSceneRoot))
  ;[1 1 1] Object Inspection
  (Utilities|FlowControl|DoOnce false
    (:Completed
      (Variables|Default|SetOriginalLocation (.location _returnvalue))
      (Variables|Default|SetOriginalRotation (.rotation _returnvalue))
      (Variables|Default|SetInspecting true)
      (Transformation|AttachComponentToComponent self (Variables|/Script/Engine.PlayerCameraManager|GetTransformComponent (Game|GetPlayerCameraManager 0)) "None" "KeepWorld" "KeepWorld" "KeepWorld" true)
      (Components|MoveComponentTo _defaultsceneroot "70.000000,20.000000,-20.000000" (Variables|/Script/Engine.SceneComponent|GetRelativeRotation _defaultsceneroot) false false 0.3 false)
      (Input|EnableInput (Game|GetPlayerController 0))
      (CallFunction|ToggleDOF true)
      (CallFunction|ToggleDetailPanel true))))

(event Input|ActionEvents|InputActionCancel
  (params (Key :type Key%20Structure))
  (bind _returnvalue (Transformation|GetActorTransform))
  (bind _defaultsceneroot (Variables|Default|GetDefaultSceneRoot))
  ;[1 1 1] Object Inspection
  (:Pressed
    (Variables|Default|SetInspecting false)
    (Transformation|DetachFromActor self "KeepWorld" "KeepWorld" "KeepWorld")
    (Input|DisableInput (Game|GetPlayerController 0))
    (CallFunction|ToggleDOF false)
    (CallFunction|ToggleDetailPanel false)
    (Components|MoveComponentTo (Variables|Default|GetDefaultSceneRoot) (Variables|Default|GetOriginalLocation) (Variables|Default|GetOriginalRotation) false false 0.3 false)
    (Utilities|FlowControl|DoOnce false) ; enters at Reset
  ))

(event Input|AxisEvents|InputAxisTurn
  (params (AxisValue :type Float%20%28single-precision%29))
  ;[1 1 1] Inspection Rotation
  (Transformation|AddLocalRotation (Variables|Default|GetDefaultSceneRoot) (Math|Rotator|MakeRotator 0.0 0.0 AxisValue) false false))

(event Input|AxisEvents|InputAxisLookUp
  (params (AxisValue :type Float%20%28single-precision%29))
  ;[1 1 1] Inspection Rotation
  (Transformation|AddLocalRotation (Variables|Default|GetDefaultSceneRoot) (Math|Rotator|MakeRotator AxisValue 0.0 0.0) false false))

(fn ConstructionScript)

(fn ToggleDOF
  (params (Enable/Disable :type Boolean))
  (bind _pp_volume (Variables|Default|GetPP_Volume))
  ;[1 1 1] Blur Settings
  (if Enable/Disable
    (bind _structout (Utilities|Struct|SetmembersinPostProcessSettings (Variables|/Script/Engine.PostProcessVolume|GetSettings _pp_volume) 3e+01 0.03 1e+02))
    (Variables|/Script/Engine.PostProcessVolume|SetSettings _pp_volume _structout)
    (else
      (bind _structout_2 (Utilities|Struct|SetmembersinPostProcessSettings (Variables|/Script/Engine.PostProcessVolume|GetSettings _pp_volume) 0.0))
      (Variables|/Script/Engine.PostProcessVolume|SetSettings _pp_volume _structout_2))))

(fn ToggleDetailPanel
  (params (Enable/Disable :type Boolean))
  ;[1 1 1] DetailedPanelObject
  (if Enable/Disable
    (Utilities|IsValid (Variables|Default|GetWidget)
      (:Is%20Valid
        _)
      (:Is%20Not%20Valid
        (bind _returnvalue (UserInterface|CreateWidget "/Game/SpectareFolder/Blueprints/ObjectDetails/WDG_ObjectDetails.WDG_ObjectDetails_C" (Game|GetPlayerController 0)))
        (Variables|Default|SetWidget _returnvalue)))
    (Default|InitializeWidget (Variables|Default|GetWidget) (Variables|Default|GetObjectName) (Variables|Default|GetObjectDetails))
    (UserInterface|Viewport|AddtoViewport (Variables|Default|GetWidget) 0)
    (else
      (Utilities|IsValid (Variables|Default|GetWidget)
        (:Is%20Valid
          (Widget|RemovefromParent (Variables|Default|GetWidget)))))))